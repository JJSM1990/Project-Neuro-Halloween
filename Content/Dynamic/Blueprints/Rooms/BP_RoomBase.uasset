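; Base room Blueprint that notifies the player character when it enters the room so the camera can adapt to that room.
; An overlap on RoomOutline, or a check shortly after BeginPlay for a player already inside, calls PlayerEnteredRoom.
; That function casts to BP_PlayerCharacter and calls NewRoom, passing the CameraMovement component's world transform as camera base and the component itself as limits, with debug prints for the cast result.
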(event `self.ReceiveBeginPlay`
  (bind _overlappingactors (`PrimitiveComponent.GetOverlappingActors` (`self.RoomOutline`) "/Game/Dynamic/Blueprints/BP_PlayerCharacter.BP_PlayerCharacter_C"))
  (`KismetSystemLibrary.Delay` 0.2)
  (if (> (`KismetArrayLibrary.Array_Length` _overlappingactors) 0)
    (`self.PlayerEnteredRoom` (`|GetArrayItem` _overlappingactors))))

(event `self.RoomOutline.OnComponentBeginOverlap`
  (params (OverlappedComponent :type "PrimitiveComponent Object Reference") (OtherActor :type "Actor Object Reference") (OtherComp :type "PrimitiveComponent Object Reference") (OtherBodyIndex :type Integer) (bFromSweep :type Boolean) (SweepResult :type "HitResult Structure (by ref)"))
  (`self.PlayerEnteredRoom` OtherActor))

(fn `PlayerEnteredRoom`
  (params (Object :type "Object Object Reference"))
  (bind _cameramovement (`self.CameraMovement`))
  (bind _asbp_player_character (cast `/Game/Dynamic/Blueprints/BP_PlayerCharacter` Object)
    (:`then`
      (`PlayerCharacter.NewRoom` _asbp_player_character (`SceneComponent.K2_GetComponentToWorld` _cameramovement) _cameramovement)
      (`KismetSystemLibrary.PrintString` "Cast Succesfull"))
    (:`CastFailed`
      (`KismetSystemLibrary.PrintString` "Cast Failed"))))

(fn `UserConstructionScript`)