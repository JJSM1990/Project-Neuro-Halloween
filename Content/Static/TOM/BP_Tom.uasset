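; BP_Tom is an unfinished actor Blueprint for the Tom character, with animation scaffolding but no working behavior.
; AnimStateMachine maps IsWalking to a state for a Select, but both branches set the same state, the options are empty and the idle and walking assets are unused.
; UpdateAnimation is empty, and the velocity-based walk check and timeline-driven Plane bounce attempt are disconnected.
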(event `UpdateAnimation`)

(fn `Anim State Machine`
  (params (isWalking :type Boolean))
  (returns (NewParam :type "PaperFlipbook Object Reference"))
  (if isWalking
    (set `self.AnimationState` 0)
    (else
      (set `self.AnimationState` 0)))
  (return (select `byte` (`self.AnimationState`) :`0` null :`1` null :`2` null :`3` null :`4` null :`5` null :`6` null :!type "PaperFlipbook Object Reference")))

(fn `UserConstructionScript`)